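; Arcane Shards gameplay ability that shows a magic circle, waits for an input press, then casts a series of shards at the targeted mouse location.
; A spawned BP_PointCollection supplies randomly rotated ground points while the avatar faces the target and plays the cast montage.
; The montage's gameplay event hides the circle and starts a looping timer that fires a gameplay cue and debug sphere per point.
; After the last point, it destroys the collection and ends.
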(event `self.K2_ActivateAbility`
  (`|ExecutionSequence`
    (:`then_0`
      (message `PlayerInterface.ShowMagicCircle` (`self.GetAvatarActorFromActorInfo`) null))
    (:`then_1`
      (`AbilityTask_WaitInputPress.WaitInputPress` false
        (:`OnPress`
          (bind (_asynctaskproxy _datahandle) (`TargetDataUnderMouse.CreateTargetDataUnderMouse`)
            (:`ValidData`
              (set `self.MouseHitLocation` (`.ImpactPoint` (`GameplayStatics.BreakHitResult` (`AbilitySystemBlueprintLibrary.GetHitResultFromTargetData` _datahandle))))
              (`|ExecutionSequence`
                (:`then_0`
                  (bind _returnvalue (`|SpawnActorFromClass` "/Game/Blueprints/AbilitySystem/Aura/Abilities/Arcane/ArcaneShards/BP_PointCollection.BP_PointCollection_C" (`KismetMathLibrary.MakeTransform` (`self.MouseHitLocation`)) "Undefined" "MultiplyWithRoot" null null))
                  (set `self.PointCollection` _returnvalue)
                  (set `self.GroundPointsArr` (`PointCollection.GetGroundPoints` _returnvalue (`self.MouseHitLocation`) (`self.Num Points`) (`KismetMathLibrary.RandomFloatInRange` 0.0 360.0)))
                  (message `CombatInterface.UpdateFacingTarget` (`self.GetAvatarActorFromActorInfo`) (`self.MouseHitLocation`)))
                (:`then_1`
                  (`AbilityTask_PlayMontageAndWait.CreatePlayMontageAndWaitProxy` "None" "/Game/Assets/Characters/Aura/Animations/Abilities/AM_Cast_ArcaneShards.AM_Cast_ArcaneShards"
                    (:`then`
                      (`AbilityTask_WaitGameplayEvent.WaitGameplayEvent` (struct :`TagName` "Event.Montage.ArcaneShards") null
                        (:`EventReceived`
                          (bind _returnvalue_2 (`KismetSystemLibrary.K2_SetTimerDelegate` (delegate `SpawnShard`) (`self.ShardSpawnDeltaTime`) true))
                          (set `self.SpawnShardTimer` _returnvalue_2)
                          (message `PlayerInterface.HideMagicCircle` (`self.GetAvatarActorFromActorInfo`))
                          (`self.SpawnShard`))))))))))))))

(event `SpawnShard`
  (if (< (`self.Count`) (`self.Num Points`))
    (bind _output_get (set `self.ShardSpawnLocation` (`SceneComponent.K2_GetComponentLocation` (`|GetArrayItem` (`self.GroundPointsArr`) (`self.Count`)))))
    (`KismetSystemLibrary.DrawDebugSphere` _output_get 20.0 12 (struct :`R` 1.0 :`G` 1.0 :`B` 1.0 :`A` 1.0) 10.0)
    (`/Engine/EditorBlueprintResources/StandardMacros.IncrementInt` (`self.Count`)
      (:`  `
        (`self.K2_ExecuteGameplayCueWithParams` (struct :`TagName` "GameplayCue.ArcaneShards") (`AbilitySystemBlueprintLibrary.MakeGameplayCueParameters` 0.0 0.0 (struct) (struct) (struct) (struct) (struct) (`self.ShardSpawnLocation`)))))
    (else
      (`KismetSystemLibrary.K2_ClearAndInvalidateTimerHandle` (`self.SpawnShardTimer`))
      (`KismetSystemLibrary.Delay` 0.2)
      (`Actor.K2_DestroyActor` (`self.PointCollection`))
      (`self.K2_EndAbility`))))