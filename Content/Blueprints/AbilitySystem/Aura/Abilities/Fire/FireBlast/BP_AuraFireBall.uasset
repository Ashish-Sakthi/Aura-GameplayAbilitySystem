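; Projectile actor for Aura's FireBlast fireball, flying outward like a boomerang and exploding on its return.
; On the server, one timeline lerps it forward to an apex, then a second homes it back to ReturnToActor's current location.
; Within ExplosionDistance it calls OnHit, applies radial damage to nearby live players except its owner, with knockback and death impulse pitched 45 degrees, then destroys itself.
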(event `self.StartOutgoingTimeline`
  (bind _array (`|MakeArray` (`self.GetOwner`)))
  (`/Engine/EditorBlueprintResources/ActorMacros.Switch Has Authority`
    (:`Authority`
      (set `self.InitialLocation` (`self.K2_GetActorLocation`))
      (set `self.ApexLocation` (+ (`self.InitialLocation`) (* (`self.GetActorForwardVector`) (`self.TravelDistance`))))
      (bind (_direction _outgoingtrack) (`Timeline|OutGoingTimeline`)
        (:`Update`
          (`self.K2_SetActorLocation` (`KismetMathLibrary.VLerp` (`self.InitialLocation`) (`self.ApexLocation`) _outgoingtrack)))
        (:`Finished`
          (bind (_direction_2 _returning) (`Timeline|ReturningTimeline`)
            (:`Update`
              (`self.K2_SetActorLocation` (`KismetMathLibrary.VLerp` (`self.ApexLocation`) (`self.K2_GetActorLocation` (`self.ReturnToActor`)) _returning))
              (if (`self.IsWithinExplodeDistance`)
                (`self.OnHit`)
                (`KismetArrayLibrary.Array_Add` _array self)
                (bind _outoverlappingactors (`AuraAbilitySystemLibrary.GetLivePlayersWithinRadius` self _array 300.0 (`self.K2_GetActorLocation`)))
                (set `self.OverlapingActors` _outoverlappingactors)
                (`AuraAbilitySystemLibrary.SetIsRadialDamageEffectParam` (`self.ExplosionDamageParams`) true 50.0 300.0 (`self.K2_GetActorLocation`))
                (for _array_element (`self.OverlapingActors`)
                  (`AuraAbilitySystemLibrary.SetTargetEffectParamsASC` (`self.ExplosionDamageParams`) (`AbilitySystemBlueprintLibrary.GetAbilitySystemComponent` _array_element))
                  (set `self.KnockbackDirection` (- (`self.K2_GetActorLocation` _array_element) (`self.K2_GetActorLocation`)))
                  (`AuraAbilitySystemLibrary.SetKnockbackDirection` (`self.ExplosionDamageParams`) (`self.OverrideKnockbackPitch`) 800.0)
                  (`AuraAbilitySystemLibrary.SetDeathImpulseDirection` (`self.ExplosionDamageParams`) (`self.OverrideKnockbackPitch`) 800.0)
                  (`AuraAbilitySystemLibrary.ApplyDamageEffect` (`self.ExplosionDamageParams`)))
                (`self.K2_DestroyActor`)))))))))

(fn `IsWithinExplodeDistance`
  (returns (ReturnValue :type Boolean))
  (return (<= (`KismetMathLibrary.VSize` (- (`self.K2_GetActorLocation`) (`self.K2_GetActorLocation` (`self.ReturnToActor`)))) (`self.ExplosionDistance`))))

(fn `OverrideKnockbackPitch`
  (returns (ReturnValue :type "Vector Structure"))
  (bind (_returnvalue_roll _returnvalue_pitch _returnvalue_yaw) (`KismetMathLibrary.BreakRotator` (`KismetMathLibrary.MakeRotFromX` (`self.KnockbackDirection`))))
  (return (`KismetMathLibrary.GetForwardVector` (`KismetMathLibrary.MakeRotator` _returnvalue_roll 45.0 _returnvalue_yaw))))

(fn `UserConstructionScript`)