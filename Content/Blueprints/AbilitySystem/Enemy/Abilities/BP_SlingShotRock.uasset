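; BP_SlingShotRock is the slingshot rock actor for an enemy ability, giving the rock mesh a random tumbling spin.
; BeginPlay picks random pitch, yaw and roll rates, and Tick applies them, scaled by delta time, as local rotation on the static mesh component.
; The graph handles only this visual spin, with no movement or damage logic.
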(event `self.ReceiveBeginPlay`
  (bind _returnvalue (`KismetMathLibrary.RandomFloatInRange` -500.0 500.0))
  (set `self.PitchRotationRate` _returnvalue)
  (set `self.YawRotationRate` _returnvalue)
  (set `self.RollRotationRate` _returnvalue))

(event `self.ReceiveTick`
  (params (DeltaSeconds :type "Float (single-precision)"))
  (`SceneComponent.K2_AddLocalRotation` (`self.SM_SlingshotRock`) (`KismetMathLibrary.MakeRotator` (* DeltaSeconds (`self.RollRotationRate`)) (* (`self.PitchRotationRate`) DeltaSeconds) (* DeltaSeconds (`self.YawRotationRate`))) false false))

(fn `UserConstructionScript`)