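; BP_StairEnterance is a stair entrance actor in the Checkpoint folder that lights up when highlighted.
; Its HighlightActor and UnHighlightActor events show and hide two point lights, without propagating visibility to child components.
; It has no other logic of its own: BeginPlay and Tick are disabled, and the construction script only calls the parent.
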(event `HighlightInterface.HighlightActor`
  (`SceneComponent.SetVisibility` (`self.PointLight1`) true false)
  (`SceneComponent.SetVisibility` (`self.PointLight`) true false))

(event `HighlightInterface.UnHighlightActor`
  (`SceneComponent.SetVisibility` (`self.PointLight1`) false false)
  (`SceneComponent.SetVisibility` (`self.PointLight`) false false))

(fn `UserConstructionScript`
  (`parent.UserConstructionScript`))