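; BP_Aura_MainMenu sets up the main menu: music, UI and a spinning magic circle backdrop.
; On BeginPlay it starts the menu music and keeps a reference to it, adds WBP_MainMenu to the viewport, then switches the player to UI-only input with a visible cursor.
; Tick rolls the MagicCircle component at MagicCircleRotationRate, scaled by delta time for frame-rate-independent motion.
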(event `self.ReceiveBeginPlay`
  (bind _returnvalue (`GameplayStatics.GetPlayerController` 0))
  (bind _returnvalue_2 (`GameplayStatics.SpawnSound2D` "/Game/Assets/Sounds/Music/Music_MainMenu.Music_MainMenu" 1.0 1.0 0.0 null))
  (set `self.MainMenuSound` _returnvalue_2)
  (bind _returnvalue_3 (`|CreateWidget` "/Game/Blueprints/UI/MainMenu/WBP_MainMenu.WBP_MainMenu_C" (`GameplayStatics.GetPlayerController` 0)))
  (`UserWidget.AddToViewport` _returnvalue_3 0)
  (`WidgetBlueprintLibrary.SetInputMode_UIOnlyEx` _returnvalue null)
  (set `PlayerController.bShowMouseCursor` true _returnvalue))

(event `self.ReceiveTick`
  (params (DeltaSeconds :type "Float (single-precision)"))
  (`SceneComponent.K2_AddLocalRotation` (`self.MagicCircle`) (`KismetMathLibrary.MakeRotator` (* DeltaSeconds (`self.MagicCircleRotationRate`))) false false))

(fn `UserConstructionScript`)